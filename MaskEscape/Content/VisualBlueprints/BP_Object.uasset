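; BP_Object is a block meant to disappear when the player presses E, per its graph comment.
; On BeginPlay it binds HandleMaskToggle to the mask-state event on BP_Baymax_Character and shows itself.
; The handler prints a debug string and disables the Cube's collision on every call, since its branch is fixed to true and ignores NewState.
; The hide-actor node is unwired, so the block stays visible.
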(event Custom|HandleMaskToggle
  (params (NewState :type Boolean))
  (bind _cube (Variables|Default|GetCube))
  ;[0.15 0.15 0.15 0.5] Make the block disappear after pressing "E"
  (Development|PrintString "Hello" true true "(R=1.000000,G=0.884559,B=0.000000,A=1.000000)")
  (if true
    (Collision|SetCollisionEnabled _cube "NoCollision")
    (else
      (Collision|SetCollisionEnabled _cube "QueryAndPhysics")
      (Rendering|SetActorHiddenInGame false))))

(event EventBeginPlay
  ;[0.15 0.15 0.15 0.5] Make the block disappear after pressing "E"
  (bind _asbp_baymax_character (Utilities|Casting|CastToBP_Baymax_Character (Game|GetPlayerCharacter 0)))
  (EventDispatchers|BindEventtoOnMaskStateChanged _asbp_baymax_character (delegate Custom|HandleMaskToggle))
  (Rendering|SetActorHiddenInGame false))

(fn ConstructionScript)